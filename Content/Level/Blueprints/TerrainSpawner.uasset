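; Actor that procedurally builds an endless strip of terrain in chained chunks along the X axis.
; On BeginPlay it spawns evenly spaced rows, opening with grass, then randomly picking grass, road, water or train terrain, with grass weighted double.
; A fixed grass row partway along carries a MoreCollision trigger.
; The first ThirdPersonCharacter overlap with that trigger spawns another TerrainSpawner just past this chunk's end.
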(event `self.ReceiveBeginPlay`
  (bind (_returnvalue_x _returnvalue_y _returnvalue_z) (`KismetMathLibrary.BreakVector` (`SceneComponent.K2_GetComponentLocation` (`self.StaticMesh`))))
  (for _index (range 31)
    (set `self.SpawnLocation` (`KismetMathLibrary.MakeVector` (`KismetMathLibrary.Conv_IntToDouble` (+ (* _index 100) (`KismetMathLibrary.FTrunc` _returnvalue_x))) _returnvalue_y _returnvalue_z))
    (if (`KismetMathLibrary.InRange_IntInt` _index 0 4)
      (`|SpawnActorFromClass` "/Game/Level/Blueprints/GrassTerrain.GrassTerrain_C" (`KismetMathLibrary.MakeTransform` (`self.SpawnLocation`)) "Undefined" "OverrideRootScale" null null)
      (elif (`KismetMathLibrary.InRange_IntInt` _index 3 9)
        (switch `int` (`KismetMathLibrary.RandomIntegerInRange` 0 4) :!label _label
          (:`0`
            (`|SpawnActorFromClass` "/Game/Level/Blueprints/GrassTerrain.GrassTerrain_C" (`KismetMathLibrary.MakeTransform` (`self.SpawnLocation`)) "Undefined" "OverrideRootScale" null null))
          (:`1`
            (`|SpawnActorFromClass` "/Game/Level/Blueprints/GrassTerrain.GrassTerrain_C" (`KismetMathLibrary.MakeTransform` (`self.SpawnLocation`)) "Undefined" "OverrideRootScale" null null))
          (:`2`
            (`|SpawnActorFromClass` "/Game/Level/Blueprints/RoadTerrain.RoadTerrain_C" (`KismetMathLibrary.MakeTransform` (`self.SpawnLocation`)) "Undefined" "OverrideRootScale" null null))
          (:`3`
            (`|SpawnActorFromClass` "/Game/Level/Blueprints/WaterTerrain.WaterTerrain_C" (`KismetMathLibrary.MakeTransform` (`self.SpawnLocation`)) "Undefined" "OverrideRootScale" null null))
          (:`4`
            (`|SpawnActorFromClass` "/Game/Level/Blueprints/TrainTerrain.TrainTerrain_C" (`KismetMathLibrary.MakeTransform` (`self.SpawnLocation`)) "Undefined" "OverrideRootScale" null null)))
        (elif (== _index 10)
          (`|SpawnActorFromClass` "/Game/Level/Blueprints/GrassTerrain.GrassTerrain_C" (`KismetMathLibrary.MakeTransform` (`self.SpawnLocation`)) "Undefined" "OverrideRootScale" null null)
          (bind _returnvalue (`|SpawnActorFromClass` "/Game/Level/Blueprints/moreCollision.moreCollision_C" (`KismetMathLibrary.MakeTransform` (`self.SpawnLocation`)) "Undefined" "OverrideRootScale" null null))
          (add `self.OnActorBeginOverlap` _returnvalue (delegate `OnActorBeginOverlap_Event_0`))
          (elif (`KismetMathLibrary.InRange_IntInt` _index 10 30)
            (goto _label)))))))

(event `OnActorBeginOverlap_Event_0` :!signature `self.OnActorBeginOverlap`
  (params (OverlappedActor :type "Actor Object Reference") (OtherActor :type "Actor Object Reference"))
  (bind (_returnvalue_x _returnvalue_y _returnvalue_z) (`KismetMathLibrary.BreakVector` (`SceneComponent.K2_GetComponentLocation` (`self.StaticMesh`))))
  (cast `/Game/Level/Blueprints/ThirdPersonCharacter` OtherActor)
  (`/Engine/EditorBlueprintResources/StandardMacros.DoOnce` false
    (:`Completed`
      (bind _output_get (set `self.SpawnLocation` (`KismetMathLibrary.MakeVector` (+ _returnvalue_x 3100.0) _returnvalue_y _returnvalue_z)))
      (`|SpawnActorFromClass` "TerrainSpawner_C" (`KismetMathLibrary.MakeTransform` _output_get) "Undefined" "OverrideRootScale" null null))))

(fn `UserConstructionScript`)