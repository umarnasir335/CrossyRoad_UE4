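; Train terrain piece that periodically spawns trains from one of its two ends, Start or End.
; On BeginPlay it caches both locations, randomly picks one side for its lifetime, and starts a looping timer with a randomized interval chosen once.
; Each timer tick has a random chance to spawn a Train at that side, yawed to a fixed heading for that end.
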(event `self.ReceiveBeginPlay`
  (set `self.StartLocation` (`SceneComponent.K2_GetComponentLocation` (`self.start`)))
  (set `self.EndLocation` (`SceneComponent.K2_GetComponentLocation` (`self.end`)))
  (set `self.startingCarLocation` (`KismetMathLibrary.RandomBool`))
  (`KismetSystemLibrary.K2_SetTimerDelegate` (delegate `SpawnVehicles`) (`KismetMathLibrary.RandomFloatInRange` 2.0 3.0) true))

(event `SpawnVehicles`
  (if (`KismetMathLibrary.RandomBool`)
    (if (`self.startingCarLocation`)
      (`|SpawnActorFromClass` "/Game/Level/Blueprints/Train.Train_C" (`KismetMathLibrary.MakeTransform` (`self.StartLocation`) (struct :`Yaw` 90.0)) "Undefined" "OverrideRootScale" null null)
      (else
        (`|SpawnActorFromClass` "/Game/Level/Blueprints/Train.Train_C" (`KismetMathLibrary.MakeTransform` (`self.EndLocation`) (struct :`Yaw` 270.0)) "Undefined" "OverrideRootScale" null null)))))

(fn `UserConstructionScript`)