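; WaterTerrain is a water lane, apparently for a Frogger-style crossing game, that spawns Log actors and reacts to the player.
; At BeginPlay it randomly fixes the spawn side (Start or End, opposite yaws) and a looping timer interval.
; Each timer tick has a random chance to spawn a log.
; Two overlap boxes, each gated by DoOnce, call UpdateScore and FallInWater respectively on the ThirdPersonCharacter.
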(event `self.ReceiveBeginPlay`
  (set `self.StartLocation` (`SceneComponent.K2_GetComponentLocation` (`self.start`)))
  (set `self.EndLocation` (`SceneComponent.K2_GetComponentLocation` (`self.end`)))
  (set `self.startingCarLocation` (`KismetMathLibrary.RandomBool`))
  (`KismetSystemLibrary.K2_SetTimerDelegate` (delegate `SpawnVehicles`) (`KismetMathLibrary.RandomFloatInRange` 2.0 3.0) true))

(event `SpawnVehicles`
  (if (`KismetMathLibrary.RandomBool`)
    (if (`self.startingCarLocation`)
      (`|SpawnActorFromClass` "/Game/Level/Blueprints/Log.Log_C" (`KismetMathLibrary.MakeTransform` (`self.StartLocation`) (struct :`Yaw` 90.0)) "Undefined" "OverrideRootScale" null null)
      (else
        (`|SpawnActorFromClass` "/Game/Level/Blueprints/Log.Log_C" (`KismetMathLibrary.MakeTransform` (`self.EndLocation`) (struct :`Yaw` 270.0)) "Undefined" "OverrideRootScale" null null)))))

(event `self.Box.OnComponentBeginOverlap`
  (params (OverlappedComponent :type "PrimitiveComponent Object Reference") (OtherActor :type "Actor Object Reference") (OtherComp :type "PrimitiveComponent Object Reference") (OtherBodyIndex :type Integer) (bFromSweep :type Boolean) (SweepResult :type "HitResult Structure (by ref)"))
  (bind _asthird_person_character (cast `/Game/Level/Blueprints/ThirdPersonCharacter` OtherActor))
  (`/Engine/EditorBlueprintResources/StandardMacros.DoOnce` false
    (:`Completed`
      (`/Game/Level/Blueprints/ThirdPersonCharacter.UpdateScore` _asthird_person_character))))

(event `self.Box1.OnComponentBeginOverlap`
  (params (OverlappedComponent :type "PrimitiveComponent Object Reference") (OtherActor :type "Actor Object Reference") (OtherComp :type "PrimitiveComponent Object Reference") (OtherBodyIndex :type Integer) (bFromSweep :type Boolean) (SweepResult :type "HitResult Structure (by ref)"))
  (bind _asthird_person_character (cast `/Game/Level/Blueprints/ThirdPersonCharacter` OtherActor))
  (`/Engine/EditorBlueprintResources/StandardMacros.DoOnce` false
    (:`Completed`
      (`/Game/Level/Blueprints/ThirdPersonCharacter.FallInWater` _asthird_person_character))))

(fn `UserConstructionScript`)