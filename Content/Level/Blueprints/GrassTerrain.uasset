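; GrassTerrain is a grass terrain piece that randomly scatters trees along its length at BeginPlay.
; It steps from the Start marker along +Y, with a count based on the distance to End, and spawns a TreeSpawner at roughly one in five steps.
; The mesh hit handler casts to ThirdPersonCharacter into a DoOnce that leads nowhere; its UpdateScore call is disconnected and never runs.
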(event `self.ReceiveBeginPlay`
  (bind (_startlocation_x _startlocation_y _startlocation_z) (`KismetMathLibrary.BreakVector` (`self.StartLocation`)))
  (set `self.StartLocation` (`SceneComponent.K2_GetComponentLocation` (`self.start`)))
  (set `self.EndLocation` (`SceneComponent.K2_GetComponentLocation` (`self.end`)))
  (for _index (range (+ (`KismetMathLibrary.FTrunc` (/ (`KismetMathLibrary.Vector_Distance` (`self.StartLocation`) (`self.EndLocation`)) 85.0)) 1))
    (if (> (`KismetMathLibrary.RandomFloat`) 0.8)
      (`|SpawnActorFromClass` "/Game/Level/Blueprints/TreeSpawner.TreeSpawner_C" (`KismetMathLibrary.MakeTransform` (`KismetMathLibrary.MakeVector` _startlocation_x (`KismetMathLibrary.Conv_IntToDouble` (+ (* _index 90) (`KismetMathLibrary.FTrunc` (.y (`self.StartLocation`))))) _startlocation_z)) "Undefined" "OverrideRootScale" null null))))

(event `self.StaticMesh.OnComponentHit`
  (params (HitComponent :type "PrimitiveComponent Object Reference") (OtherActor :type "Actor Object Reference") (OtherComp :type "PrimitiveComponent Object Reference") (NormalImpulse :type "Vector Structure") (Hit :type "HitResult Structure (by ref)"))
  (bind _asthird_person_character (cast `/Game/Level/Blueprints/ThirdPersonCharacter` OtherActor))
  (`/Engine/EditorBlueprintResources/StandardMacros.DoOnce` false))

(fn `UserConstructionScript`)